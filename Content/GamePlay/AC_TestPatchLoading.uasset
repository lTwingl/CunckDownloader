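; Test actor that drives the chunk patch downloader subsystem and opens PatchTestMap when patching succeeds.
; BeginPlay binds manifest and patch completion callbacks, then creates the downloader.
; A successful manifest starts a looping timer that prints download and mount progress, clearing itself once both reach 1.0 or the actor is destroyed.
; The patch completion handler prints the result before loading the map.
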(event Custom|CustomEvent_0)

(event Custom|CustomEvent_1
  (params (Succeeded :type Boolean))
  (if Succeeded
    (bind _returnvalue (Utilities|Time|SetTimerbyFunctionName 0 "GetChunkPacthProgress" 0.1 true))
    (Variables|Default|SetNewVar_0 _returnvalue)
    (else
      (Development|PrintString (Utilities|String|Append "ManifestGetComplete" (Utilities|String|ToString(Boolean) Succeeded))))))

(event EventBeginPlay
  (bind _returnvalue (Subsystems|GetPatchDownloaderSubSystem))
  (EventDispatchers|BindEventtoOnManifestComplete _returnvalue (delegate Custom|CustomEvent_1))
  (EventDispatchers|BindEventtoOnPatchComplete _returnvalue (EventDispatchers|CreateEvent :!event ACTestPatchLoadingAutoGenFunc))
  (Class|PatchDownloaderSubSystem|CreatePatchDownloader _returnvalue))

(event Collision|EventActorBeginOverlap
  (params (OtherActor :type Actor%20Object%20Reference)))

(event EventTick
  (params (DeltaSeconds :type Float%20%28single-precision%29)))

(event EventDestroyed
  (bind _newvar_0 (Variables|Default|GetNewVar_0))
  (if (Utilities|Time|IsValidTimerHandle _newvar_0)
    (Utilities|Time|ClearandInvalidateTimerbyHandle _newvar_0)))

(fn ConstructionScript)

(fn GetChunkPacthProgress
  (bind _returnvalue (Subsystems|GetPatchDownloaderSubSystem))
  (bind _newvar_0 (Variables|Default|GetNewVar_0))
  (bind (_filesdownloaded _totalfilestodownload _downloadpercent _chunksmounted _totalchunkstomount _mountpercent) (Class|PatchDownloaderSubSystem|GetLoadingProgress _returnvalue))
  (Development|PrintString (Class|KismetStringLibrary|BuildStringDouble "" "CurrentLoadingProgress:" _downloadpercent "%"))
  (Development|PrintString (Class|KismetStringLibrary|BuildStringDouble "" "CurrentMountingProgress:" _mountpercent "%"))
  (if (and (>= _mountpercent 1.0) (>= _downloadpercent 1.0))
    (if (Utilities|Time|IsValidTimerHandle _newvar_0)
      (Utilities|Time|ClearandInvalidateTimerbyHandle _newvar_0))))

(fn ACTestPatchLoadingAutoGenFunc
  (params (Succeeded :type Boolean))
  (Development|PrintString (Utilities|String|Append "OnReceivePatchComplete:" (Utilities|String|ToString(Boolean) Succeeded)))
  (if Succeeded
    (Game|OpenLevel(byName) "PatchTestMap")))