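; Test actor that, on BeginPlay, shows the main panel widget and spawns a set of actors, apparently for checking patch content.
; It prints a debug message, adds WBP_MainPanel to the viewport, then spawns each class in the ActorClass array in a row along Y.
; It then swaps its own StaticMesh to NewMesh.
; A material override node exists but is never executed.
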(event EventBeginPlay
  (Development|PrintString "ShowMainPanel" true true "(R=1.000000,G=0.216748,B=0.186899,A=1.000000)" 11.0)
  (Utilities|FlowControl|Sequence
    (:then_0
      (bind _returnvalue (UserInterface|CreateWidget "/Game/TestData_2/WBP_MainPanel.WBP_MainPanel_C"))
      (UserInterface|Viewport|AddtoViewport _returnvalue 0))
    (:then_1
      (for (_array_element _array_index) (Variables|Default|GetActorClass)
        (Game|SpawnActorfromClass _array_element (Math|Transform|MakeTransform (Math|Vector|MakeVectorNetQuantize 0.0 (Math|Conversions|ToFloat(Integer) (* _array_index 100)) 1e+02)) "Undefined" 0 0))
      (Components|StaticMesh|SetStaticMesh (Variables|Default|GetStaticMesh) (Utilities|ResolveSoftReference (Variables|Default|GetNew%20Mesh))))))

(event Collision|EventActorBeginOverlap
  (params (OtherActor :type Actor%20Object%20Reference)))

(event EventTick
  (params (DeltaSeconds :type Float%20%28single-precision%29)))

(fn ConstructionScript)